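; BP_PlacementManager runs cursor-driven building placement, from spawning a ghost preview through rotation to confirmation.
; While placing, Tick snaps the ghost's X/Y to the tile size and swaps building and footprint grid materials according to its validation result.
; Confirming a valid placement spawns a hard-coded BP_BuildingTownhall at the unsnapped cursor hit, destroys the ghost, records the building and begins construction with the selected data.
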(event EventBeginPlay
  (bind _asbp_player_controller (Utilities|Casting|CastToBP_PlayerController (Game|GetPlayerController 0)))
  (Variables|Default|SetPlayer%20Controller _asbp_player_controller)
  (bind _asbp_game_instance (Utilities|Casting|CastToBP_GameInstance (Game|GetGameInstance)))
  (Variables|Default|SetGame%20Instance _asbp_game_instance))

(event Collision|EventActorBeginOverlap
  (params (OtherActor :type Actor%20Object%20Reference)))

(event EventTick
  (params (DeltaSeconds :type Float%20%28single-precision%29))
  (if (Variables|Default|GetIsPlacing)
    (CallFunction|UpdatePlacement)))

(fn ConstructionScript)

(fn UpdatePlacement
  (bind _currentghost (Variables|Default|GetCurrentGhost))
  (bind _playercontroller (Variables|Default|GetPlayerController))
  (bind _tilesize (Variables|Default|GetTileSize))
  (bind _currentghost_2 (Variables|Default|GetCurrentGhost))
  (bind _hitresult (Game|Player|GetHitResultUnderCursorbyChannel _playercontroller "TraceTypeQuery4" true))
  (bind (_bblockinghit _binitialoverlap _time _distance _location _impactpoint) (Collision|BreakHitResult _hitresult))
  (bind (_x _y _z) (Math|Vector|BreakVector _location))
  (if (not (or (== _tilesize 0.0) (== _x 0.0)))
    (bind _output_get (LocalVariables|SetSnappedLocation (Math|Vector|MakeVector (* (Math|Float|Round (/ _x _tilesize)) (Variables|Default|GetTileSize)) (* (Math|Float|Round (/ _y (Variables|Default|GetTileSize))) (Variables|Default|GetTileSize)) _z)))
    (Transformation|SetActorLocation (Variables|Default|GetCurrentGhost) _output_get false false)
    (bind _isvalid (Default|ValidatePlacement (Variables|Default|GetCurrentGhost)))
    (bind _output_get_2 (Variables|Default|SetPlacementIsValid _isvalid))
    (if _output_get_2
      (Rendering|Material|SetMaterial (Variables|/Game/Core/Blueprints/Actors/Ghost/BP_GhostBuildingBase.BP_GhostBuildingBase_C|GetBuildingMesh _currentghost) 0 (Variables|/Game/Core/Blueprints/Actors/Ghost/BP_GhostBuildingBase.BP_GhostBuildingBase_C|GetBuildingValidMat _currentghost))
      (for _array_element (Actor|GetAllChildActors (Variables|/Game/Environment/Grid/BP_Grid.BP_Grid_C|GetGridVisual (Variables|/Game/Core/Blueprints/Actors/Ghost/BP_GhostBuildingBase.BP_GhostBuildingBase_C|GetFootprintGrid _currentghost)) true)
        (Rendering|Material|SetMaterial (Variables|/Game/Environment/Grid/BP_GridMeshInst.BP_GridMeshInst_C|GetInstancedStaticMesh (.AsBP%20Ghost%20Grid%20Mesh%20Inst (Utilities|Casting|CastToBP_GhostGridMeshInst _array_element))) 0 (Variables|/Game/Core/Blueprints/Actors/Ghost/BP_GhostBuildingBase.BP_GhostBuildingBase_C|GetGridValidMat _currentghost)))
      (else
        (Rendering|Material|SetMaterial (Variables|/Game/Core/Blueprints/Actors/Ghost/BP_GhostBuildingBase.BP_GhostBuildingBase_C|GetBuildingMesh _currentghost_2) 0 (Variables|/Game/Core/Blueprints/Actors/Ghost/BP_GhostBuildingBase.BP_GhostBuildingBase_C|GetBuildingInvalidMat _currentghost_2))
        (for _array_element_2 (Actor|GetAllChildActors (Variables|/Game/Environment/Grid/BP_Grid.BP_Grid_C|GetGridVisual (Variables|/Game/Core/Blueprints/Actors/Ghost/BP_GhostBuildingBase.BP_GhostBuildingBase_C|GetFootprintGrid _currentghost_2)) true)
          (Rendering|Material|SetMaterial (Variables|/Game/Environment/Grid/BP_GridMeshInst.BP_GridMeshInst_C|GetInstancedStaticMesh (.AsBP%20Ghost%20Grid%20Mesh%20Inst (Utilities|Casting|CastToBP_GhostGridMeshInst _array_element_2))) 0 (Variables|/Game/Core/Blueprints/Actors/Ghost/BP_GhostBuildingBase.BP_GhostBuildingBase_C|GetGridInvalidMat _currentghost_2)))))))

(fn StartPlacement
  (params (Data :type S%20Building%20Data%20Structure))
  (CallFunction|LogText "Starting placement")
  (Variables|Default|SetCurrentBuildingData Data)
  (if (not (Variables|Default|GetIsPlacing))
    (Variables|Default|SetIsPlacing true)
    (bind _asbp_player_controller (Utilities|Casting|CastToBP_PlayerController (Game|GetPlayerController 0)))
    (bind _output_get (Variables|Default|SetPlayerController _asbp_player_controller))
    (bind _returnvalue (Game|SpawnActorfromClass (.ghostclass (Variables|Default|GetCurrentBuildingData)) (Math|Transform|MakeTransform (Math|Vector|MakeVector (.x (.Location (Collision|BreakHitResult (.HitResult (Game|Player|GetHitResultUnderCursorbyChannel _output_get "TraceTypeQuery1" true))))) (.y (.Location (Collision|BreakHitResult (.HitResult (Game|Player|GetHitResultUnderCursorbyChannel _output_get "TraceTypeQuery1" true))))) (.z (.ImpactPoint (Collision|BreakHitResult (.HitResult (Game|Player|GetHitResultUnderCursorbyChannel _output_get "TraceTypeQuery1" true)))))) "0, 0, 0" "1.000000,1.000000,1.000000") "AlwaysSpawn" "MultiplyWithRoot" self 0))
    (Variables|Default|SetCurrentGhost _returnvalue)))

(fn ConfirmPlacement
  (bind _playercontroller (Variables|Default|GetPlayerController))
  (bind _hitresult (Game|Player|GetHitResultUnderCursorbyChannel _playercontroller "TraceTypeQuery1" true))
  (bind _location (Collision|BreakHitResult _hitresult))
  (if (Variables|Default|GetPlacementIsValid)
    (bind _returnvalue (Game|SpawnActorfromClass "/Game/Core/Blueprints/Actors/Buildings/Townhall/BP_BuildingTownhall.BP_BuildingTownhall_C" (Math|Transform|MakeTransform (Math|Vector|MakeVector (.x _location) (.y _location) (+ (.z _location) 2e+01)) (Transformation|GetActorRotation (Variables|Default|GetCurrentGhost)) "1.000000,1.000000,1.000000") "AlwaysSpawn" "MultiplyWithRoot" self 0))
    (Actor|DestroyActor (Variables|Default|GetCurrentGhost))
    (Rendering|SetVisibility (Variables|/Game/Environment/Grid/BP_Grid.BP_Grid_C|GetChildActor_GridVisual (Variables|/Game/Core/Blueprints/Actors/Buildings/BP_BuildingBase.BP_BuildingBase_C|GetGrid _returnvalue)) false false)
    (Variables|Default|SetIsPlacing false)
    (Utilities|Array|Add (Variables|Default|GetPlacedBuildings) _returnvalue)
    (bind _valuepin (Utilities|Map|ForEachLoop(Map) (Variables|/Game/Environment/Grid/BP_Grid.BP_Grid_C|GetGridTileMap (Variables|/Game/Core/Blueprints/Actors/Buildings/BP_BuildingBase.BP_BuildingBase_C|GetGrid _returnvalue)))
      (:then
        (bind _result (Math|Integer|IncrementInt (.BuildingID (Utilities|Struct|BreakS_TileData _valuepin)))
          (:%20%20
            (Utilities|Struct|SetmembersinS_TileData (Utilities|Struct|MakeS_TileData (.Index (Utilities|Struct|BreakS_TileData _valuepin)) (.Transform (Utilities|Struct|BreakS_TileData _valuepin)) (.TileMesh (Utilities|Struct|BreakS_TileData _valuepin)) (.TileMaterial (Utilities|Struct|BreakS_TileData _valuepin)) (.WorldLocation (Utilities|Struct|BreakS_TileData _valuepin)) (.TileInst (Utilities|Struct|BreakS_TileData _valuepin)) _result)))))
      (:CompletedPin
        (Default|BeginConstruction _returnvalue (Variables|Default|GetCurrentBuildingData))))
    (else
      (Development|PrintString "um, no"))))

(fn RotateGhost
  (bind _output_get (Variables|Default|SetRotationIndex (Math|Integer|%(Integer) (+ (Variables|Default|GetRotationIndex) 1) 4)))
  (Transformation|SetActorRotation (Variables|Default|GetCurrentGhost) (Math|Rotator|MakeRotator 0.0 0.0 (Math|Conversions|ToFloat(Integer) (Utilities|Select :Index _output_get :Option%200 0 :Option%201 90 :Option%202 180 :Option%203 270))))
  (Default|ValidatePlacement (Variables|Default|GetCurrentGhost)))