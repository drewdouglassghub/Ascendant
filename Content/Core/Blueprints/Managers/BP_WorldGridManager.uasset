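; World grid manager that tracks which tiles are occupied by placed actors such as buildings.
; It converts world locations to tile coordinates and back to tile centers using TileSize, and computes footprint origins centered on a location.
; OccupyGrid loops over a footprint and registers each cell's occupancy type and actor in GridCellMap, with debug prints.
; Lookups read that map, which holds only registered cells, and the occupancy check prints a message for missing ones.
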(event EventBeginPlay)

(event Collision|EventActorBeginOverlap
  (params (OtherActor :type Actor%20Object%20Reference)))

(event EventTick
  (params (DeltaSeconds :type Float%20%28single-precision%29)))

(fn ConstructionScript)

(fn WorldtoGrid
  (params (WorldLocation :type Vector))
  (return (Utilities|Struct|MakeIntPoint (Math|Float|Floor (/ (.x WorldLocation) (Variables|Default|GetTileSize))) (Math|Float|Floor (/ (.y WorldLocation) (Variables|Default|GetTileSize))))))

(fn GridtoWorld
  (params (GridCoordinate :type Int%20Point%20Structure))
  (return (Math|Vector|MakeVector (+ (* (.x GridCoordinate) (Variables|Default|GetTileSize)) (/ (Variables|Default|GetTileSize) 2.0)) (+ (* (.y GridCoordinate) (Variables|Default|GetTileSize)) (/ (Variables|Default|GetTileSize) 2.0)) 0.0)))

(fn IsCellOccupied
  (params (GridCoordinate :type Int%20Point%20Structure))
  (bind _gridcellmap (Variables|Default|GetGridCellMap))
  (if (Utilities|Map|Contains _gridcellmap GridCoordinate)
    (if (Utilities|Enum|NotEqual(Enum) (.OccupancyType (Utilities|Struct|BreakS_GridCell (.Value (Utilities|Map|Find _gridcellmap GridCoordinate)))) "NewEnumerator0")
      (return true)
      (else
        (return false)))
    (else
      (Development|PrintString "World Grid Cell doesn't exist"))))

(fn GetCell
  (params (Coordinate :type Int%20Point%20Structure))
  (bind _gridcellmap (Variables|Default|GetGridCellMap))
  (bind (_value _returnvalue) (Utilities|Map|Find _gridcellmap Coordinate))
  (return _returnvalue _value))

(fn RegisterCell
  (params (Coordinate :type Int%20Point%20Structure) (CellData :type S%20Grid%20Cell%20Structure) (BuildingData :type S%20Building%20Data%20Structure))
  (Development|PrintString "setting world cell" true true "(R=1.000000,G=0.357731,B=0.001283,A=1.000000)" 5.0)
  (Development|PrintString (Utilities|String|ToString(Integer) Coordinate) true true "(R=1.000000,G=0.452348,B=0.003546,A=1.000000)" 5.0)
  (Development|PrintString (Utilities|String|Append "Placed building " (Utilities|GetDisplayName (.occupancyactor CellData)) "at coordinate " (Utilities|String|ToString(Integer) Coordinate) "with occupancy of " (Utilities|String|EnumtoString (.occupancytype CellData))) true true "(R=1.000000,G=0.440883,B=0.000000,A=1.000000)" 5.0)
  (Utilities|Map|Add (Variables|Default|GetGridCellMap) Coordinate (Utilities|Struct|MakeS_GridCell (.occupancytype CellData) (.occupancyactor CellData)))
  (CallFunction|LogInteger "World Grid Size " (Utilities|Map|Length (Variables|Default|GetGridCellMap))))

(fn OccupyGrid
  (params (ActorRef :type Actor%20Object%20Reference) (Footprint :type Int%20Point%20Structure) (Origin :type Vector))
  (Variables|Default|SetOrigin Origin)
  (for _index (range 0 (- (.x Footprint) 1))
    (bind _output_get (LocalVariables|SetCurrentX (+ (.x (Variables|Default|GetOrigin)) _index)))
    (for _index_2 (range 0 (- (.y Footprint) 1))
      (bind _output_get_2 (LocalVariables|SetCurrentY (+ (.y (Variables|Default|GetOrigin)) _index_2)))
      (bind _output_get_3 (LocalVariables|SetCoordinate (Utilities|Struct|MakeIntPoint (Math|Float|Truncate _output_get) (Math|Float|Truncate _output_get_2))))
      (Development|PrintString (Utilities|String|Append (Utilities|GetDisplayName ActorRef) (Utilities|String|ToString(Integer) _output_get_3)))
      (CallFunction|RegisterCell _output_get_3 (Utilities|Struct|MakeS_GridCell "NewEnumerator1" ActorRef)))))

(fn CalculateOrigin
  (params (WorldLocation :type Vector) (FootprintX :type Integer) (FootprintY :type Integer))
  (bind _gridcoordinate (CallFunction|WorldtoGrid WorldLocation))
  (return (Math|Vector|MakeVector (Math|Conversions|ToFloat(Integer) (- (.x _gridcoordinate) (Math|Float|Floor (Math|Conversions|ToFloat(Integer) (/ FootprintX 2))))) (Math|Conversions|ToFloat(Integer) (- (.y _gridcoordinate) (Math|Float|Floor (Math|Conversions|ToFloat(Integer) (/ FootprintY 2))))) 0.0)))