(event Input|EnhancedActionEvents|EnhancedInputActionIA_Spin
  (params (ActionValue :type Float%20%28double-precision%29) (ElapsedSeconds :type Float%20%28double-precision%29) (TriggeredSeconds :type Float%20%28double-precision%29) (InputAction :type Input%20Action%20Object%20Reference :default "/Game/Core/Blueprints/Player/EnhancedActions/Input/IA_Spin.IA_Spin"))
  (bind _plyrpwn (Variables|Default|GetPlyrPwn))
  (bind _springarm (Variables|/Game/Core/Blueprints/Player/BP_Pawn.BP_Pawn_C|GetSpringArm _plyrpwn))
  (bind _relativerotation (Variables|/Script/Engine.SceneComponent|GetRelativeRotation _springarm))
  ;[1 0.06771 0.06771] Spin
  (Transformation|AddLocalRotation _springarm (Math|Rotator|MakeRotator 0.0 0.0 ActionValue) false false)
  (Transformation|SetRelativeRotation _springarm (Math|Rotator|MakeRotator 0.0 (Math|Float|ClampAngle (.pitch _relativerotation) -5e+01 -1e+01) (.yaw _relativerotation)) false false))

(event Input|EnhancedActionEvents|EnhancedInputActionIA_MoveCamera
  (params (ActionValue :type Vector%202D%20Structure) (ElapsedSeconds :type Float%20%28double-precision%29) (TriggeredSeconds :type Float%20%28double-precision%29) (InputAction :type Input%20Action%20Object%20Reference :default "/Game/Core/Blueprints/Player/EnhancedActions/Input/IA_MoveCamera.IA_MoveCamera"))
  (bind _plyrpwn (Variables|Default|GetPlyrPwn))
  (bind _springarm (Variables|/Game/Core/Blueprints/Player/BP_Pawn.BP_Pawn_C|GetSpringArm _plyrpwn))
  (bind _returnvalue (Transformation|GetWorldRotation _springarm))
  (bind _returnvalue_2 (Math|Rotator|MakeRotator 0.0 0.0 (.yaw _returnvalue)))
  ;[1 0.016 0.016] Move
  (Pawn|Input|AddMovementInput _plyrpwn (Math|Vector|GetForwardVector _returnvalue_2) (.x ActionValue) true)
  (Pawn|Input|AddMovementInput _plyrpwn (Math|Vector|GetRightVector _returnvalue_2) (.y ActionValue) true))

(event Input|EnhancedActionEvents|EnhancedInputActionIA_Zoom
  (params (ActionValue :type Float%20%28double-precision%29) (ElapsedSeconds :type Float%20%28double-precision%29) (TriggeredSeconds :type Float%20%28double-precision%29) (InputAction :type Input%20Action%20Object%20Reference :default "/Game/Core/Blueprints/Player/EnhancedActions/Input/IA_Zoom.IA_Zoom"))
  (bind _plyrpwn (Variables|Default|GetPlyrPwn))
  ;[1 0.04167 0.04167] Zoom
  (Variables|/Game/Core/Blueprints/Player/BP_Pawn.BP_Pawn_C|SetZoom%20Direction _plyrpwn ActionValue)
  (Default|UpdateZoom _plyrpwn)
  (Default|Dof _plyrpwn))

(event Input|EnhancedActionEvents|EnhancedInputActionIA_Look
  (params (ActionValue :type Float%20%28double-precision%29) (ElapsedSeconds :type Float%20%28double-precision%29) (TriggeredSeconds :type Float%20%28double-precision%29) (InputAction :type Input%20Action%20Object%20Reference :default "/Game/Core/Blueprints/Player/EnhancedActions/Input/IA_Look.IA_Look"))
  (bind _plyrpwn (Variables|Default|GetPlyrPwn))
  (bind _springarm (Variables|/Game/Core/Blueprints/Player/BP_Pawn.BP_Pawn_C|GetSpringArm _plyrpwn))
  (bind _relativerotation (Variables|/Script/Engine.SceneComponent|GetRelativeRotation _springarm))
  ;[0.9635 0 0.00936] Look Up
  (bind _result (Math|Float|NegateFloat ActionValue)
    (:%20%20
      (Transformation|AddLocalRotation _springarm (Math|Rotator|MakeRotator 0.0 _result 0.0) false false)
      (Transformation|SetRelativeRotation _springarm (Math|Rotator|MakeRotator 0.0 (Math|Float|ClampAngle (.pitch _relativerotation) -5e+01 -1e+01) (Math|Float|ClampAngle (.yaw _relativerotation) -9e+01 9e+01)) false false))))

(event Input|EnhancedActionEvents|EnhancedInputActionIA_Select
  (params (ActionValue :type Boolean) (ElapsedSeconds :type Float%20%28double-precision%29) (TriggeredSeconds :type Float%20%28double-precision%29) (InputAction :type Input%20Action%20Object%20Reference :default "/Game/Core/Blueprints/Player/EnhancedActions/Input/IA_Select.IA_Select"))
  (bind (_hitresult _returnvalue) (Game|Player|GetHitResultUnderCursorbyChannel "TraceTypeQuery6" true))
  ;[0.15 0.15 0.15 0.5] SELECT
  (if _returnvalue
    (bind _out (CallFunction|LogObject "Object clicked -> " (.HitActor (Collision|BreakHitResult _hitresult))))
    (Utilities|IsValid _out
      (:Is%20Valid
        (if (Utilities|DoesObjectImplementInterface _out "/Game/Core/Utilities/BPI_Interactable.BPI_Interactable_C")
          (bind _newparam (Class|BPIInteractable|GetInteractableType(Message) _out))
          (switch Utilities|FlowControl|Switch|SwitchonE_Interactables _newparam
            (:NewEnumerator0
              (Development|PrintString "Hello, you have found a building"))
            (:NewEnumerator1
              (Development|PrintString "Hello, you have found a Resource"))
            (:NewEnumerator2
              (Development|PrintString "Hello, you have found a Shrine"))
            (:NewEnumerator3
              (Development|PrintString "Hello, you have found a Follower")))
          (else
            (CallFunction|LogText "Not Interactable"))))
      (:Is%20Not%20Valid
        (CallFunction|LogObject "Invalid: " _out)))))

(event Input|EnhancedActionEvents|EnhancedInputActionIA_Build
  (params (ActionValue :type Boolean) (ElapsedSeconds :type Float%20%28double-precision%29) (TriggeredSeconds :type Float%20%28double-precision%29) (InputAction :type Input%20Action%20Object%20Reference :default "/Game/Core/Blueprints/Player/EnhancedActions/Input/IA_Build.IA_Build"))
  ;[0.15 0.15 0.15 0.5] BUILD
  (:Completed
    (if (not (Variables|/Game/Core/Blueprints/Managers/BP_PlacementManager.BP_PlacementManager_C|GetIsPlacing (Variables|/Game/Core/Blueprints/Game/BP_GameInstance.BP_GameInstance_C|GetPlacementManager (Variables|Default|GetGameInstance))))
      (bind _aswbp_base_window (Utilities|Casting|CastToWBP_BaseWindow (.Value (Utilities|Map|Find (Variables|/Game/Core/Blueprints/Game/BP_GameInstance.BP_GameInstance_C|GetActiveWidgetMap (Variables|Default|GetGameInstance)) "NewEnumerator4"))))
      (Default|ShowBuildMenu _aswbp_base_window))))

(event Input|EnhancedActionEvents|EnhancedInputActionIA_ConfirmPlacement
  (params (ActionValue :type Boolean) (ElapsedSeconds :type Float%20%28double-precision%29) (TriggeredSeconds :type Float%20%28double-precision%29) (InputAction :type Input%20Action%20Object%20Reference :default "/Game/Core/Blueprints/Player/EnhancedActions/Input/IA_ConfirmPlacement.IA_ConfirmPlacement"))
  (bind _placementmanager (Variables|Default|GetPlacementManager))
  ;[0.15 0.15 0.15 0.5] PLACEMENT
  (:Completed
    (Development|PrintString "Placed")
    (if (Variables|/Game/Core/Blueprints/Managers/BP_PlacementManager.BP_PlacementManager_C|GetIsPlacing _placementmanager)
      (Default|ConfirmPlacement _placementmanager))))

(event Input|EnhancedActionEvents|EnhancedInputActionIA_RotateGhost
  (params (ActionValue :type Boolean) (ElapsedSeconds :type Float%20%28double-precision%29) (TriggeredSeconds :type Float%20%28double-precision%29) (InputAction :type Input%20Action%20Object%20Reference :default "/Game/Core/Blueprints/Player/EnhancedActions/Input/IA_RotateGhost.IA_RotateGhost"))
  (bind _placementmanager (Variables|Default|GetPlacementManager))
  ;[0.15 0.15 0.15 0.5] PLACEMENT
  (Development|PrintString "Rotating")
  (if (Variables|/Game/Core/Blueprints/Managers/BP_PlacementManager.BP_PlacementManager_C|GetIsPlacing _placementmanager)
    (Default|RotateGhost _placementmanager)))

(event EventBeginPlay
  ;[0.04566 0.07805 0.9583 0.5] Begin Play
  (Variables|Default|SetbShowMouseCursor true)
  (bind _asbp_pawn (Utilities|Casting|CastToBP_Pawn (Pawn|GetControlledPawn)))
  (Variables|Default|SetPlyrPwn _asbp_pawn)
  (bind _mainhud (CallFunction|SetMainHUD self))
  (Variables|Default|SetMainHUD _mainhud)
  (Variables|Default|SetGameInstance (.AsBP%20Game%20Instance (Utilities|Casting|CastToBP_GameInstance (Game|GetGameInstance))))
  (Variables|Default|SetGameMode (.AsBP%20Game%20Mode (Utilities|Casting|CastToBP_GameMode (Game|GetGameMode))))
  (Variables|Default|SetPlayer%20State (.AsBP%20Player%20State (Utilities|Casting|CastToBP_PlayerState (Game|GetPlayerState 0))))
  (bind _ui_manager (Default|GetUIManager (Variables|Default|GetGameInstance)))
  (Variables|Default|SetUI%20Manager _ui_manager)
  (Variables|Default|SetPlacementManager (Variables|/Game/Core/Blueprints/Game/BP_GameInstance.BP_GameInstance_C|GetPlacementManager (Variables|Default|GetGameInstance))))

(event EventTick
  (params (DeltaSeconds :type Float%20%28single-precision%29)))

(fn ConstructionScript)

(fn SetPlayerFaction
  (params (Faction :type E_Factions%20Enum :default "NewEnumerator0"))
  (Variables|Default|SetFaction Faction))