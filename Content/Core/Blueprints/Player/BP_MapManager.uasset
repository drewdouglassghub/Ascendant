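; Map manager that stores the game's grid tiles with terrain, biome and resource data, and registers itself with the game instance on construction.
; Grid spawning and ground tracing defer to the parent class.
; RegisterTileData adds tiles lying below a BiomeElevationMap threshold to GridTileMap, then initializes the child terrain visual.
; Lookups read that map by index, and cursor locations snap to staggered hex-style indices using column parity.
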(event EventBeginPlay
  (|CallParentFunction))

(event Collision|EventActorBeginOverlap
  (params (OtherActor :type Actor%20Object%20Reference))
  (|CallParentFunction OtherActor) ; This node is disabled and will not be called.\nDrag off pins to build functionality.
)

(event EventTick
  (params (DeltaSeconds :type Float%20%28single-precision%29))
  (|CallParentFunction DeltaSeconds) ; This node is disabled and will not be called.\nDrag off pins to build functionality.
)

(fn ConstructionScript
  (|CallParentFunction)
  (bind _output_get (Variables|Default|SetGame%20Instance (.AsBP%20Game%20Instance (Utilities|Casting|CastToBP_GameInstance (Game|GetGameInstance)))))
  (Default|SetMapManager _output_get))

(fn AverageHitCornerLocations
  (params (HitLocations :type Array%20of%20Vectors) (NumCorners :type Integer))
  (bind _runningtotal (LocalVariables|GetRunningTotal))
  (for _index (range 0 (- NumCorners 1))
    (Variables|Default|SetCornerHitTotal (+ (Utilities|Array|Get(acopy) HitLocations _index) (Utilities|Array|Get(acopy) _runningtotal _index)))
    (Variables|Default|SetAverageFinalLoc (/ (+ (Utilities|Array|Get(acopy) HitLocations _index) (Utilities|Array|Get(acopy) _runningtotal _index)) "5.000000,5.000000,0.000000"))
    (Utilities|Array|Add :TargetArray _runningtotal)))

(fn AverageNormalCornerLocations
  (params (NormalLocations :type Array%20of%20Vectors) (NumCorners :type Integer))
  (for (_array_element _array_index) NormalLocations
    (Utilities|Array|Add (LocalVariables|GetRunningTotal) _array_element)
    (Variables|Default|SetAvgNormal (Math|Vector|Normalize (/ (+ _array_element (Utilities|Array|Get(acopy) (LocalVariables|GetRunningTotal) _array_index)) "5.000000,5.000000,0.000000")))))

(fn TraceforGround
  (params (Location :type Vector :default "0, 0, 0") (Index :type Int%20Point%20Structure))
  (bind (_outlocation _tiletype) (|CallParentFunction Location Index))
  (return _outlocation _tiletype))

(fn NormalizeIndex
  (params (Index :type Int%20Point%20Structure) (CenterLocation :type Vector))
  (return (Math|Vector|Normalize (- (CallFunction|GetTileLocation Index) CenterLocation))))

(fn SpawnGrid
  (params (CenterLocation :type Vector :default "0, 0, 0") (TileSize :type Vector :default "0, 0, 0") (TileCount :type Int%20Point%20Structure) (Shape :type E_GridShape%20Enum :default "NewEnumerator0") (UseEnvironment :type Boolean))
  (|CallParentFunction CenterLocation TileSize TileCount Shape UseEnvironment))

(fn RegisterTileData
  (params (TileData :type S%20Tile%20Data%20Structure))
  (bind (_index _tiletype _transform _tilestate _unitsontile _height _biometype _food _energy _minerals _tileid) (Utilities|Struct|BreakS_TileData TileData))
  (bind _keypin (Utilities|Map|ForEachLoop(Map) (Variables|Default|GetBiomeElevationMap) :!label _label)
    (:then
      (if (> _keypin _height)
        (Utilities|Map|Add (Variables|Default|GetGridTileMap) _index (Utilities|Struct|MakeS_TileData _index "NewEnumerator1" _transform "NewEnumerator0" 0 _height _biometype _food _energy _minerals _tileid))
        (goto _label BreakPin)))
    (:CompletedPin
      (bind _asbp_terrain_visual (Utilities|Casting|CastToBP_TerrainVisual (Variables|/Script/Engine.ChildActorComponent|GetChildActor (Variables|Default|GetChildActor_TerrainVisual))))
      (Default|InitializeTerrainVisual _asbp_terrain_visual _index))))

(fn GetTileDatabyCoordinate
  (params (Index :type Int%20Point%20Structure))
  (return (.Value (Utilities|Map|Find (Variables|Default|GetGridTileMap) Index))))

(fn FindTileLocation
  (params (Index :type Int%20Point%20Structure))
  (return (.location (.Transform (Utilities|Struct|BreakS_TileData (.Value (Utilities|Map|Find (Variables|Default|GetGridTileMap) Index)))))))

(fn AddTerrainTile
  (params (TileData :type S%20Tile%20Data%20Structure)))

(fn GetTerrainUnderCursor
  (params (Location :type Vector))
  (Variables|Default|SetLocation%20on%20Grid (- Location (Variables|Default|GetGridBottomLeftLocation)))
  (Variables|Default|SetSnappedLocationOnGrid_0 (Math|Conversions|ToVector2D(Vector) (CallFunction|SnapVectortoVector (* (Variables|Default|GetLocation%20on%20Grid) "1.000000,2.000000,1.000000") (* (Variables|Default|GetTile%20Size) "0.750000,0.250000,1.000000"))))
  (LocalVariables|SetTempIndex (/ (Variables|Default|GetSnappedLocationOnGrid_0) (* (Math|Conversions|ToVector2D(Vector) (Variables|Default|GetTile%20Size)) "(X=0.750000,Y=1.000000)")))
  (if (CallFunction|IsFloatEven (.x (LocalVariables|GetTempIndex)))
    (return (Utilities|Struct|MakeIntPoint (Math|Float|Truncate (.x (LocalVariables|GetTempIndex))) (* (Math|Float|Round (/ (.y (LocalVariables|GetTempIndex)) 2.0)) 2)))
    (else
      (return (Utilities|Struct|MakeIntPoint (Math|Float|Truncate (.x (LocalVariables|GetTempIndex))) (+ (* (Math|Float|Floor (/ (.y (LocalVariables|GetTempIndex)) 2.0)) 2) 1))))))