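; Base building actor that constructs itself over time from BuildingData, is interactable (logging only) and exposes a "Door" socket for road connection.
; The construction script spawns a footprint-sized grid through a child BP_Grid actor.
; BeginConstruction starts a looping timer, while UpdateBuild tracks progress and swaps phase meshes at percentage thresholds.
; On completion it clears the timer, shows the final mesh and occupies its footprint in the GameInstance's WorldGridManager.
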(event Custom|UpdateBuild
  (bind _buildingdata (Variables|Default|GetBuildingData))
  (if (not (Variables|Default|GetIsBuildComplete))
    (bind _output_get (Variables|Default|SetBuildTimeRemaining (- (Variables|Default|GetBuildTimeRemaining) (.timerrate _buildingdata))))
    (CallFunction|LogFloat "" _output_get)
    (bind _output_get_2 (Variables|Default|SetBuildPercentage (- 1.0 (/ _output_get (.buildtimetotal _buildingdata)))))
    (CallFunction|CheckConstructionPhase _output_get_2)
    (if (<= (Variables|Default|GetBuildTimeRemaining) 0.0)
      (Variables|Default|SetIsBuildComplete true)
      (CallFunction|FinishConstruction))))

(event EventBeginPlay)

(event Collision|EventActorBeginOverlap
  (params (OtherActor :type Actor%20Object%20Reference)))

(event EventTick
  (params (DeltaSeconds :type Float%20%28single-precision%29)))

(event EventInteract
  (CallFunction|LogText "Building -> " "Interaction"))

(fn ConstructionScript
  (bind _buildingdata (Variables|Default|GetBuildingData))
  (bind _asbp_grid (Utilities|Casting|CastToBP_Grid (Variables|/Script/Engine.ChildActorComponent|GetChildActor (Variables|Default|GetChildActor_Grid))))
  (bind _output_get (Variables|Default|SetGrid _asbp_grid))
  (CallFunction|UpdateGridFootprint)
  (Default|SpawnGrid _output_get (Transformation|GetWorldLocation (Variables|Default|GetBuildingMesh)) (Variables|/Game/Environment/Grid/BP_Grid.BP_Grid_C|GetTile%20Size _output_get) (Utilities|Struct|MakeIntPoint (.footprintx _buildingdata) (.footprinty _buildingdata))))

(fn SetGridSize
  (bind _buildingdata (Variables|Default|GetBuildingData))
  (Variables|Default|SetGridSize (* (.footprintx _buildingdata) (.footprinty _buildingdata))))

(fn UpdateGridFootprint
  (bind (_origin _boxextent) (Collision|GetActorBounds false false))
  (bind _grid (Variables|Default|GetGrid))
  (Default|SetFootprintfromBounds _grid _origin _boxextent (.x (Variables|/Game/Environment/Grid/BP_Grid.BP_Grid_C|GetTile%20Size _grid))))

(fn BeginConstruction
  (params (BuildingData :type S%20Building%20Data%20Structure))
  (bind _output_get (Variables|Default|SetBuildingData BuildingData))
  (Variables|Default|SetBuildTimeRemaining (.BuildTimeTotal (Utilities|Struct|BreakS_BuildingData _output_get)))
  (bind _output_get_2 (Variables|Default|SetConstructionPhaseIndex 0))
  (Components|StaticMesh|SetStaticMesh (Variables|Default|GetBuildingMesh) (Utilities|Array|Get(acopy) (.PhasesMeshes (Utilities|Struct|BreakS_BuildingData _output_get)) _output_get_2))
  (bind _returnvalue (Utilities|Time|SetTimerbyEvent (EventDispatchers|CreateEvent :!event Custom|UpdateBuild) (.TimerRate (Utilities|Struct|BreakS_BuildingData _output_get)) true false (.BuildDelay (Utilities|Struct|BreakS_BuildingData _output_get))))
  (Variables|Default|SetBuildTimer _returnvalue))

(fn CheckConstructionPhase
  (params (Percentage :type Float%20%28double-precision%29))
  (bind _buildingdata (Variables|Default|GetBuildingData))
  (bind (_name _icon _ghostclass _buildingclass _cost _description _category _buildtimetotal _phasethresholds _phasesmeshes) (Utilities|Struct|BreakS_BuildingData _buildingdata))
  (for (_array_element _array_index) _phasethresholds
    (if (< _array_element Percentage)
      (if (!= (Variables|Default|GetConstructionPhaseIndex) _array_index)
        (bind _output_get (Variables|Default|SetConstructionPhaseIndex _array_index))
        (Components|StaticMesh|SetStaticMesh (Variables|Default|GetBuildingMesh) (Utilities|Array|Get(acopy) _phasesmeshes _output_get))))))

(fn FinishConstruction
  (bind _returnvalue (Game|GetGameInstance))
  (bind _buildingdata (Variables|Default|GetBuildingData))
  (bind _buildingdata_2 (Variables|Default|GetBuildingData))
  (bind _phasesmeshes (Utilities|Struct|BreakS_BuildingData _buildingdata))
  (bind (_name _icon _ghostclass _buildingclass _cost _description _category _buildtimetotal _phasethresholds _phasesmeshes_2 _constructionphasetotal _timerrate _builddelay _footprintx _footprinty) (Utilities|Struct|BreakS_BuildingData _buildingdata_2))
  (bind _asbp_game_instance (Utilities|Casting|CastToBP_GameInstance _returnvalue))
  (bind _worldgridmanager (Variables|/Game/Core/Blueprints/Game/BP_GameInstance.BP_GameInstance_C|GetWorldGridManager _asbp_game_instance))
  (Utilities|Time|ClearandInvalidateTimerbyHandle (Variables|Default|GetBuildTimer))
  (Components|StaticMesh|SetStaticMesh (Variables|Default|GetBuildingMesh) (Utilities|Array|Get(acopy) _phasesmeshes (- (Utilities|Array|Length _phasesmeshes) 1)))
  (bind _origin (Default|CalculateOrigin _worldgridmanager (Transformation|GetActorLocation) _footprintx _footprinty))
  (Default|OccupyGrid _worldgridmanager 0 (Utilities|Struct|MakeIntPoint _footprintx _footprinty) _origin))

(fn SetFootprintfromBounds
  (params (Origin :type Vector) (BoxExtent :type Vector) (TileSize :type Float%20%28double-precision%29))
  (Variables|Default|SetMin (- Origin BoxExtent))
  (Variables|Default|SetMax (+ Origin BoxExtent))
  (CallFunction|LogInteger "X " (+ (- (Math|Float|Floor (/ (.x (Variables|Default|GetMax)) (Variables|Default|GetTileSize))) (Math|Float|Floor (/ (.x (Variables|Default|GetMin)) (Variables|Default|GetTileSize)))) 1))
  (CallFunction|LogInteger "Y " (+ (- (Math|Float|Floor (/ (.y (Variables|Default|GetMax)) (Variables|Default|GetTileSize))) (Math|Float|Floor (/ (.y (Variables|Default|GetMin)) (Variables|Default|GetTileSize)))) 1)))

(fn GetRoadConnectionPoint
  (return (Transformation|GetSocketTransform (Variables|Default|GetBuildingMesh) "Door" "RTS_World")))

(fn CanInteract
  (return true))

(fn GetInteractableType
  (CallFunction|LogText "Type ->" "Building")
  (return "NewEnumerator0"))

(fn GetInteractionLocation
  (return (Transformation|GetWorldLocation (Variables|Default|GetBuildingMesh))))