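; Base ghost actor for building placement, showing a footprint grid and checking whether the spot is valid.
; Construction caches the placement manager from BP_GameMode, has the child BP_Grid derive its footprint from actor bounds, then spawns tiles using CurrentBuildingData's footprint size.
; ValidatePlacement runs two downward box traces on separate channels, passing only when no grid or building is hit and terrain is.
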(event EventBeginPlay)

(event Collision|EventActorBeginOverlap
  (params (OtherActor :type Actor%20Object%20Reference)))

(event EventTick
  (params (DeltaSeconds :type Float%20%28single-precision%29)))

(fn ConstructionScript
  (bind _currentbuildingdata (Variables|Default|GetCurrentBuildingData))
  (bind (_name _icon _ghostclass _buildingclass _cost _description _category _buildtimetotal _phasethresholds _phasesmeshes _constructionphasetotal _timerrate _builddelay _footprintx _footprinty) (Utilities|Struct|BreakS_BuildingData _currentbuildingdata))
  (bind _asbp_game_mode (Utilities|Casting|CastToBP_GameMode (Game|GetGameMode)))
  (bind _output_get (Variables|Default|SetGame%20Mode _asbp_game_mode))
  (Variables|Default|SetPlacement%20Manager (Variables|/Game/Core/Blueprints/Game/BP_GameMode.BP_GameMode_C|GetPlacementManager _output_get))
  (bind _asbp_grid (Utilities|Casting|CastToBP_Grid (Variables|/Script/Engine.ChildActorComponent|GetChildActor (Variables|Default|GetChildActor_Grid))))
  (bind _output_get_2 (Variables|Default|SetFootprintGrid _asbp_grid))
  (CallFunction|UpdateGridFootprint)
  (Default|SpawnGrid (Variables|Default|GetFootprintGrid) (Transformation|GetWorldLocation (Variables|Default|GetBuildingMesh)) (Variables|/Game/Environment/Grid/BP_Grid.BP_Grid_C|GetTile%20Size _output_get_2) (Utilities|Struct|MakeIntPoint _footprintx _footprinty)))

(fn UpdateGridFootprint
  (bind (_origin _boxextent) (Collision|GetActorBounds false false))
  (Default|SetFootprintfromBounds (Variables|Default|GetFootprintGrid) _origin _boxextent (Variables|Placement|GetTileSize)))

(fn ValidatePlacement
  (bind _footprintgrid (Variables|Default|GetFootprintGrid))
  (bind (_origin _boxextent) (Collision|GetActorBounds _footprintgrid false false))
  (LocalVariables|SetFootprintOrigin _origin)
  (LocalVariables|SetFootprintExtent _boxextent)
  (bind _valid (CallFunction|ValidateFootprint))
  (return _valid))

(fn ValidateFootprint
  (LocalVariables|SetIsValidPlacement true)
  (CallFunction|TraceforGridorBuilding)
  (CallFunction|TraceforTerrain)
  (if (and (Variables|Default|GetNoGridPlaced) (Variables|Default|GetTerrainValid))
    (return true)
    (else
      (return false))))

(fn TraceforGridorBuilding
  (bind _returnvalue (Transformation|GetActorLocation))
  (bind _bounds (Variables|Default|GetBounds))
  (bind _returnvalue_2 (Components|Box|GetScaledBoxExtent _bounds))
  (bind (_outhit _returnvalue_3) (Collision|BoxTraceByChannel (Math|Vector|MakeVector (.x _returnvalue) (.y _returnvalue) (.z _returnvalue)) (Math|Vector|MakeVector (.x _returnvalue) (.y _returnvalue) -7.5e+04) (Math|Vector|MakeVector (.x _returnvalue_2) (.y _returnvalue_2) (.z _returnvalue_2)) (Transformation|GetActorRotation) "TraceTypeQuery3" true 0 "None"))
  (if _returnvalue_3
    (Variables|Default|SetNoGridPlaced false)
    (else
      (Variables|Default|SetNoGridPlaced true))))

(fn TraceforTerrain
  (bind _returnvalue (Transformation|GetActorLocation))
  (bind _returnvalue_2 (Collision|BoxTraceByChannel (Math|Vector|MakeVector (.x _returnvalue) (.y _returnvalue) (.z _returnvalue)) (Math|Vector|MakeVector (.x _returnvalue) (.y _returnvalue) -7.5e+04) (Components|Box|GetScaledBoxExtent (Variables|Default|GetBounds)) (Transformation|GetActorRotation) "TraceTypeQuery4" true (Variables|Default|GetActors%20to%20Ignore) "None" true "(R=1.000000,G=0.000000,B=0.000000,A=1.000000)" "(R=0.000000,G=1.000000,B=0.000000,A=1.000000)" 0.0))
  (if _returnvalue_2
    (Variables|Default|SetTerrainValid true)
    (else
      (Variables|Default|SetTerrainValid false))))

(fn SetFootprintfromBounds
  (params (Origin :type Vector) (BoxExtent :type Vector) (TileSize :type Float%20%28double-precision%29))
  (Variables|Default|SetMin (- Origin BoxExtent))
  (Variables|Default|SetMax (+ Origin BoxExtent))
  (bind _out (CallFunction|LogInteger "GHOST X " (+ (- (Math|Float|Floor (/ (.x (Variables|Default|GetMax)) (Variables|Placement|GetTileSize))) (Math|Float|Floor (/ (.x (Variables|Default|GetMin)) (Variables|Placement|GetTileSize)))) 1)))
  (bind _out_2 (CallFunction|LogInteger "GHOST Y " (+ (- (Math|Float|Floor (/ (.y (Variables|Default|GetMax)) (Variables|Placement|GetTileSize))) (Math|Float|Floor (/ (.y (Variables|Default|GetMin)) (Variables|Placement|GetTileSize)))) 1)))
  (Variables|Default|SetCurrentBuildingData (Utilities|Struct|MakeS_BuildingData "" 0 0 0 0 "" "NewEnumerator0" 0.0 0 0 0 0.0 0.0 _out _out_2 Origin)))