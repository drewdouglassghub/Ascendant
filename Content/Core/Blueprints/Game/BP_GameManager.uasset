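; BP_GameManager is a Blueprint that sets up the game's starting state on BeginPlay and kicks off the AI opponents.
; It caches the game mode, game instance and player controller, and flags the game mode as being in colony placement.
; TriggerAIOpponents hands off to the game instance through CallOnAITriggered.
; All setup stops if the game mode is not a BP_GameMode.
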(event EventBeginPlay
  (bind _asbp_game_mode (Utilities|Casting|CastToBP_GameMode (Game|GetGameMode)))
  (bind _output_get (Variables|Default|SetGame%20Mode _asbp_game_mode))
  (Variables|/Game/Core/Blueprints/Game/BP_GameMode.BP_GameMode_C|SetIsPlacingColony _output_get true)
  (Variables|Default|SetGameInstance (.AsBP%20Game%20Instance (Utilities|Casting|CastToBP_GameInstance (Game|GetGameInstance))))
  (Variables|Default|SetPlayer%20Controller (.AsBP%20Player%20Controller (Utilities|Casting|CastToBP_PlayerController (Game|GetPlayerController 0))))
  (CallFunction|TriggerAIOpponents))

(event Collision|EventActorBeginOverlap
  (params (OtherActor :type Actor%20Object%20Reference)))

(event EventTick
  (params (DeltaSeconds :type Float%20%28single-precision%29)))

(fn ConstructionScript)

(fn TriggerAIOpponents
  (Default|CallOnAITriggered (Variables|Default|GetGameInstance)))