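; Game mode Blueprint that initializes the game's core managers on BeginPlay and caps the frame rate at a low fixed limit.
; It caches the player controller and game instance, then stores the AI, UI, placement and world grid managers returned by the instance's setter functions.
; A second step loops over the factions enum, setting the game, AI and UI managers each pass without using the faction value.
; A RecastNavMesh lookup is left unconnected.
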(event EventBeginPlay
  (bind _returnvalue (Settings|GetGameUserSettings))
  (Class|GameUserSettings|SetFrameRateLimit _returnvalue 2e+01)
  (Utilities|FlowControl|Sequence
    (:then_0
      (Variables|Default|SetPlayer%20Controller (.AsBP%20Player%20Controller (Utilities|Casting|CastToBP_PlayerController (Game|GetPlayerController 0))))
      (bind _asbp_game_instance (Utilities|Casting|CastToBP_GameInstance (Game|GetGameInstance)))
      (bind _output_get (Variables|Default|SetGameInstance _asbp_game_instance))
      (bind _aimanager (Default|SetAIManager _output_get))
      (Variables|Managers|SetAIManager _aimanager)
      (bind _uimanager (Default|SetUIManager _output_get))
      (Variables|Managers|SetUI%20Manager _uimanager)
      (bind _placementmanager (Default|SetPlacementManager _output_get))
      (Variables|Default|SetPlacementManager _placementmanager)
      (bind _worldgridmanager (Default|SetWorldGridManager _output_get))
      (Variables|Default|SetWorldGridManager _worldgridmanager))
    (:then_1
      (|ForEachE_Factions
        (:LoopBody
          (bind _gamemanager (Default|SetGameManager (Variables|Default|GetGameInstance)))
          (Variables|Managers|SetGameManager _gamemanager)
          (bind _aimanager_2 (Default|SetAIManager (Variables|Default|GetGameInstance)))
          (Variables|Managers|SetAIManager _aimanager_2)
          (bind _uimanager_2 (Default|SetUIManager (Variables|Default|GetGameInstance)))
          (Variables|Managers|SetUI%20Manager _uimanager_2))))))

(event EventTick
  (params (DeltaSeconds :type Float%20%28single-precision%29)))

(fn ConstructionScript)