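; BP_WorldGenerator is an unfinished world generator that builds height map data for a square world.
; GenerateWorld clears HeightMap, then loops over WorldSize in X and Y, appending 1D Perlin noise remapped to 0–1.
; Each cell's noise input is a whole number combining both coordinates, with X scaled by a large stride.
; The nested chunk loops and GenerateChunk are empty, and no event here calls GenerateWorld.
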(event EventBeginPlay)

(event Collision|EventActorBeginOverlap
  (params (OtherActor :type Actor%20Object%20Reference)))

(event EventTick
  (params (DeltaSeconds :type Float%20%28single-precision%29)))

(fn ConstructionScript)

(fn GenerateWorld
  (Utilities|Array|Clear (Variables|Default|GetHeightMap))
  (for _index (range 0 (- (Variables|Default|GetWorldSize) 1))
    (LocalVariables|SetX _index)
    (for _index_2 (range 0 (- (Variables|Default|GetWorldSize) 1))
      (bind _output_get (LocalVariables|SetY _index_2))
      (bind _output_get_2 (Variables|Default|SetNoiseInput (Math|Conversions|ToFloat(Integer) (+ (LocalVariables|GetY) (* (LocalVariables|GetX) 10000)))))
      (bind _output_get_3 (Variables|Default|SetNoiseValue (Class|KismetMathLibrary|PerlinNoise1D _output_get_2)))
      (Utilities|Array|Add (Variables|Default|GetHeightMap) (* (+ _output_get_3 1.0) 0.5))
      (for _index_3 (range 0 (- (Variables|Default|GetNumChunksX) 1))
        (for _index_4 (range 0 (- (Variables|Default|GetNumChunksY) 1))
          _)))))

(fn GenerateChunk)