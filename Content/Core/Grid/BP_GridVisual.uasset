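; Visual layer for a grid, drawing its tiles as flat-mesh instances through a child BP_GridMeshInst actor.
; Initialization takes the current shape's mesh and material from the Grid, applies a ground offset and resets the lowest Z.
; Tile updates remove the instance by index and re-add it only for walkable tile types.
; Destruction clears the main and tactical instances; resetting lowest Z also clears the tactical-generation flag.
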(event EventBeginPlay)

(event Collision|EventActorBeginOverlap
  (params (OtherActor :type Actor%20Object%20Reference)))

(event EventTick
  (params (DeltaSeconds :type Float%20%28single-precision%29)))

(fn ConstructionScript)

(fn DestroyGridVisual
  (bind _gridmeshinst (Variables|Default|GetGridMeshInst))
  (bind _grid_mesh_inst_tactical (Variables|Default|GetGrid%20Mesh%20Inst%20Tactical))
  (Utilities|FlowControl|Sequence
    (:then_0
      (Utilities|IsValid _gridmeshinst
        (:Is%20Valid
          (Default|ClearInstance _gridmeshinst))))
    (:then_1
      (Utilities|IsValid _grid_mesh_inst_tactical
        (:Is%20Valid
          (Default|ClearInstance _grid_mesh_inst_tactical))))
    (:then_2
      (CallFunction|SetGridLowestZ 9.9999e+05))))

(fn SetGridLowestZ
  (params (GridLowestZ :type Float%20%28double-precision%29))
  (Variables|Default|SetGridLowestZ GridLowestZ)
  (Variables|Default|SetNeedToGenerateTactical false))

(fn UpdateTileVisual
  (params (Data :type S%20Tile%20Data%20Structure))
  (Utilities|FlowControl|Sequence
    (:then_0
      (Default|RemoveInstance (Variables|Default|GetGridMeshInst) (.index Data))
      (if (CallFunction|IsTileWalkable (.tiletype Data))
        (Default|AddInstance (Variables|Default|GetGridMeshInst) (.index Data) (.transform Data) "NewEnumerator0" (.tiletype Data))))))

(fn SetOffsetfromGround
  (params (Offset :type Float%20%28double-precision%29))
  (Variables|Default|SetOffsetFromGround Offset)
  (Transformation|SetRelativeLocation (Variables|Default|GetChildActor_GridMeshInst) (Math|Conversions|ToVector(Float) (Variables|Default|GetOffsetFromGround)) false false))

(fn InitializeGridVisual
  (params (Grid :type BP%20Grid%20Object%20Reference))
  (Variables|Default|SetGrid Grid)
  (Variables|Default|SetGridMeshInst (.AsBP%20Grid%20Mesh%20Inst (Utilities|Casting|CastToBP_GridMeshInst (Variables|/Script/Engine.ChildActorComponent|GetChildActor (Variables|Default|GetChildActor_GridMeshInst)))))
  (Default|InitializeGridMeshInst (Variables|Default|GetGridMeshInst) (.flatmesh (Default|GetCurrentShapeData (Variables|Default|GetGrid))) (.flatmaterial (Default|GetCurrentShapeData (Variables|Default|GetGrid))) false "QueryOnly")
  (CallFunction|SetOffsetfromGround (Variables|Default|GetOffsetFromGround))
  (CallFunction|SetGridLowestZ 9.9999e+05))