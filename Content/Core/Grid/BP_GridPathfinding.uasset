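; A* pathfinder for a tile grid of squares, hexagons or triangles, finding a path or reachable tiles within a length limit.
; Neighbors are filtered by tile type and occupancy, then queued in a cost-sorted open list using movement cost, a shape-specific distance heuristic and a diagonal tie-breaker.
; The search can spread across delayed, time-budgeted iterations, broadcasting data updates, clearing and completion through events.
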(event Custom|FindPathWithDelay
  (Utilities|FlowControl|Sequence
    (:then_0
      (goto _label_3 Open))
    (:then_1
      (Variables|Default|SetLoopStartTime (Math|DateTime|Now) :!label _label)
      (if (> (Utilities|Array|Length (Variables|Default|GetDiscoveredTileIndices)) 0) :!label _label_2
        (bind _foundtargettile (CallFunction|AnalyzeNextDiscoveredTile))
        (if _foundtargettile
          (bind _path (CallFunction|GeneratePath))
          (Default|CallOnPathfindingCompleted _path)
          (else
            (if (> (Variables|Default|GetMaxMs) 0.0)
              (if (< (Class|KismetMathLibrary|GetTotalMilliseconds (- (Math|DateTime|Now) (Variables|Default|GetLoopStartTime))) (Variables|Default|GetMaxMs))
                (goto _label_2)
                (else
                  _)))
            (Utilities|FlowControl|RetriggerableDelay (Variables|Default|GetDelayBetweenIteration))
            (Utilities|FlowControl|Gate true :!label _label_3
              (:Exit
                (goto _label)))))
        (else
          ;[1 1 1] No possible path
          (Default|CallOnPathfindingCompleted (select (Variables|Default|GetReturnReachables) (Variables|Default|GetAnalyzedTileIndices) (Utilities|Array|MakeArray ""))))))))

(event Custom|CloseDelayGate
  (Utilities|FlowControl|Gate true) ; enters at Close
)

(event EventBeginPlay)

(event Collision|EventActorBeginOverlap
  (params (OtherActor :type Actor%20Object%20Reference)))

(event EventTick
  (params (DeltaSeconds :type Float%20%28single-precision%29)))

(fn ConstructionScript)

(fn GetValidTileNeighbors
  (params (Index :type Int%20Point%20Structure) (IncludeDiagonals :type Boolean) (ValidTypes :type Array%20of%20E_TileType%20Enums :default "NewEnumerator0"))
  (LocalVariables|SetInputData (.Value (Utilities|Map|Find (Variables|/Game/Blueprints/BP_Grid.BP_Grid_C|GetGridTileMap (Variables|Default|GetGrid)) Index)))
  (bind _neighbors (CallFunction|GetNeighborIndexes Index IncludeDiagonals))
  (for _array_element _neighbors
    (LocalVariables|SetData (.Value (Utilities|Map|Find (Variables|/Game/Blueprints/BP_Grid.BP_Grid_C|GetGridTileMap (Variables|Default|GetGrid)) _array_element)))
    (if (Utilities|Array|ContainsItem (Variables|Default|GetValid%20Types) (.tiletype (LocalVariables|GetData)))
      (if (not (Utilities|IsValid (Utilities|Array|Get(acopy) (.unitsontile (LocalVariables|GetData)))))
        (if (<= (Math|Float|Absolute(Float) (- 0.0 0.0)) (.x (Variables|/Game/Blueprints/BP_Grid.BP_Grid_C|GetTile%20Size (Variables|Default|GetGrid))))
          (Utilities|Array|Add (LocalVariables|GetRet) (Utilities|Struct|MakeS_PathfindingData "(X=-999,Y=-999)" (CallFunction|GetTileTypeMoveCost (.tiletype (LocalVariables|GetData))) 999999 999999 Index))))))
  (return 0))

(fn GetNeighborIndexes
  (params (Index :type Int%20Point%20Structure) (IncludeDiagonals :type Boolean))
  (switch Utilities|FlowControl|Switch|SwitchonE_GridShape (Variables|/Game/Blueprints/BP_Grid.BP_Grid_C|GetShape (Variables|Default|GetGrid))
    (:NewEnumerator1
      (return (CallFunction|GetNeigborIndexesSquare Index IncludeDiagonals)))
    (:NewEnumerator2
      (return (CallFunction|GetNeigborIndexesHexagon Index)))
    (:NewEnumerator3
      (return (CallFunction|GetNeigborIndexesTriangle Index IncludeDiagonals)))))

(fn GetNeigborIndexesSquare
  (params (Index :type Int%20Point%20Structure) (IncludeDiagonals :type Boolean))
  (bind _intpoint (Utilities|Struct|MakeIntPoint 1 0))
  (bind _intpoint_2 (Utilities|Struct|MakeIntPoint 0 1))
  (bind _intpoint_3 (Utilities|Struct|MakeIntPoint -1 0))
  (bind _intpoint_4 (Utilities|Struct|MakeIntPoint 0 -1))
  (bind _returnvalue (+ Index _intpoint))
  (bind _returnvalue_2 (+ Index _intpoint_2))
  (bind _returnvalue_3 (+ Index _intpoint_3))
  (bind _returnvalue_4 (+ Index _intpoint_4))
  (bind _array (Utilities|Array|MakeArray _returnvalue _returnvalue_2 _returnvalue_3 _returnvalue_4))
  (if IncludeDiagonals
    (LocalVariables|SetRet _array)
    (Utilities|Array|AppendArray (LocalVariables|GetRet) (Utilities|Array|MakeArray (+ Index (Utilities|Struct|MakeIntPoint 1 1)) (+ Index (Utilities|Struct|MakeIntPoint -1 1)) (+ Index (Utilities|Struct|MakeIntPoint 1 -1)) (+ Index (Utilities|Struct|MakeIntPoint -1 -1))))
    (return (LocalVariables|GetRet))
    (else
      (return _array))))

(fn GetNeigborIndexesHexagon
  (params (Index :type Int%20Point%20Structure))
  (return (Utilities|Array|MakeArray (+ Index (Utilities|Struct|MakeIntPoint 1 1)) (+ Index (Utilities|Struct|MakeIntPoint 0 2)) (+ Index (Utilities|Struct|MakeIntPoint -1 1)) (+ Index (Utilities|Struct|MakeIntPoint -1 -1)) (+ Index (Utilities|Struct|MakeIntPoint 0 -2)) (+ Index (Utilities|Struct|MakeIntPoint 1 -1)))))

(fn GetNeigborIndexesTriangle
  (params (Index :type Int%20Point%20Structure) (IncludeDiagonals :type Boolean))
  (LocalVariables|SetRet (Utilities|Array|MakeArray (+ Index (Utilities|Struct|MakeIntPoint 0 -1)) (+ Index (Utilities|Struct|MakeIntPoint 0 1)) "" ""))
  (if true
    (Utilities|Array|Add (LocalVariables|GetRet) (+ Index (Utilities|Struct|MakeIntPoint -1 0)))
    (else
      (Utilities|Array|Add (LocalVariables|GetRet) (+ Index (Utilities|Struct|MakeIntPoint 1 0)))))
  (if IncludeDiagonals
    (if true
      (Utilities|Array|AppendArray (LocalVariables|GetRet) (Utilities|Array|MakeArray (+ Index (Utilities|Struct|MakeIntPoint 1 0)) (+ Index (Utilities|Struct|MakeIntPoint -1 2)) (+ Index (Utilities|Struct|MakeIntPoint -1 -2))))
      (else
        (Utilities|Array|AppendArray (LocalVariables|GetRet) (Utilities|Array|MakeArray (+ Index (Utilities|Struct|MakeIntPoint -1 0)) (+ Index (Utilities|Struct|MakeIntPoint 1 2)) (+ Index (Utilities|Struct|MakeIntPoint 1 -2))))))
    (return (LocalVariables|GetRet))
    (else
      (return (LocalVariables|GetRet)))))

(fn IsInputDataValid
  (bind _grid (Variables|Default|GetGrid))
  (bind _target (Variables|Default|GetTarget))
  (bind _gridtilemap (Variables|/Game/Blueprints/BP_Grid.BP_Grid_C|GetGridTileMap _grid))
  (bind _value (Utilities|Map|Find _gridtilemap _target))
  (bind (_index _tiletype _transform _tilestate _unitsontile) (Utilities|Struct|BreakS_TileData _value))
  (if (!= (Variables|Default|GetStart) (Variables|Default|GetTarget))
    (if true
      (if (not (Variables|Default|GetReturnReachables))
        (if (Default|IsTileWalkable (Variables|Default|GetGrid) (Variables|Default|GetTarget))
          (if (<= (CallFunction|GetMinimumCostBetweenTiles (Variables|Default|GetStart) (Variables|Default|GetTarget) (Variables|Default|GetDiagonals)) (Variables|Default|GetPathLength))
            (if (Utilities|Array|ContainsItem (Variables|Default|GetValid%20Types) _tiletype)
              (if (not (Utilities|IsValid (Utilities|Array|Get(acopy) _unitsontile)))
                (return true)
                (else
                  (return false)))
              (else
                (return false)))
            (else
              (return false)))
          (else
            (return false)))
        (else
          (return true)))
      (else
        (return false)))
    (else
      (return false))))

(fn GetMinimumCostBetweenTiles
  (params (Index%201 :type Int%20Point%20Structure) (Index%202 :type Int%20Point%20Structure) (Diagonals :type Boolean))
  (bind _returnvalue (- Index%201 Index%202))
  (bind _returnvalue_2 (- Index%201 Index%202))
  (bind _returnvalue_3 (< (.x Index%202) (.x Index%201)))
  (bind _returnvalue_4 (< (.x Index%202) (.x Index%201)))
  (bind _returnvalue_5 (- Index%201 Index%202))
  (bind _returnvalue_6 (- Index%201 Index%202))
  (bind _returnvalue_7 (- Index%201 Index%202))
  (bind _returnvalue_8 (Math|Integer|SelectInt 1 -1 _returnvalue_4))
  (switch Utilities|FlowControl|Switch|SwitchonE_GridShape (Variables|/Game/Blueprints/BP_Grid.BP_Grid_C|GetShape (Variables|Default|GetGrid))
    (:NewEnumerator1
      ;[1 1 1] Cost For Square
      (if Diagonals
        (return (Math|Integer|Max(Integer) (Math|Integer|Absolute(Integer) (.x _returnvalue_7)) (Math|Integer|Absolute(Integer) (.y _returnvalue_7))))
        (else
          (return (+ (Math|Integer|Absolute(Integer) (.x _returnvalue_5)) (Math|Integer|Absolute(Integer) (.y _returnvalue_5)))))))
    (:NewEnumerator2
      ;[1 1 1] Cost for Hexagon
      (return (+ (.x _returnvalue) (Math|Integer|Max(Integer) (/ (- (.y _returnvalue) (.x _returnvalue)) 2)))))
    (:NewEnumerator3
      (if Diagonals
        ;[1 1 1] Triangles with diagonals
        (return (/ (+ (Math|Integer|Absolute(Integer) (.x _returnvalue_6)) (Math|Integer|Absolute(Integer) (.y _returnvalue_6))) 2))
        (else
          (LocalVariables|SetX (Math|Integer|Absolute(Integer) (.x _returnvalue_2)))
          (LocalVariables|SetY (Math|Integer|Absolute(Integer) (.y _returnvalue_2)))
          (if (select false (select _returnvalue_3 (<= (- (LocalVariables|GetX) 1) (LocalVariables|GetY)) (<= (LocalVariables|GetX) (LocalVariables|GetY))) (select _returnvalue_3 (<= (LocalVariables|GetX) (LocalVariables|GetY)) (<= (- (LocalVariables|GetX) 1) (LocalVariables|GetY))))
            (return (+ (LocalVariables|GetX) (LocalVariables|GetY)))
            (elif true
              (return (* (LocalVariables|GetX) 2))
              (else
                (return (+ (* (LocalVariables|GetX) 2) (Math|Integer|SelectInt (* _returnvalue_8 -1) _returnvalue_8 false)))))))))))

(fn FindPath
  (params (Start :type Int%20Point%20Structure) (Target :type Int%20Point%20Structure) (Diagonals :type Boolean) (ValidTypes :type Array%20of%20E_TileType%20Enums :default "NewEnumerator0") (Delay :type Float%20%28double-precision%29) (MaxMs :type Float%20%28double-precision%29) (ReturnReachables :type Boolean) (PathLength :type Integer))
  ;[1 1 1] Set Variables
  (Variables|Default|SetStart Start)
  (Variables|Default|SetTarget Target)
  (Variables|Default|SetDiagonals Diagonals)
  (Variables|Default|SetValid%20Types ValidTypes)
  (Variables|Default|SetDelayBetweenIteration Delay)
  (Variables|Default|SetMaxMs MaxMs)
  (Variables|Default|SetReturnReachables ReturnReachables)
  (Variables|Default|SetPathLength PathLength))

(fn AnalyzeNextDiscoveredTile
  (bind _tilepathdata (CallFunction|PullCheapestTilefromDiscoveredList))
  (Default|CallOnPathfindingDataUpdated (.Index (Utilities|Struct|BreakS_PathfindingData _tilepathdata)))
  (bind _neighbors (CallFunction|GetValidTileNeighbors :IncludeDiagonals (Variables|Default|GetDiagonals) :ValidTypes (Variables|Default|GetValid%20Types)))
  (while (> (Utilities|Array|Length _neighbors) 0)
    _))

(fn GeneratePath
  (LocalVariables|SetCurrent (Variables|Default|GetTarget))
  (while (!= (LocalVariables|GetCurrent) (Variables|Default|GetStart))
    (Utilities|Array|Add (LocalVariables|GetInvertedPath) (LocalVariables|GetCurrent))
    (LocalVariables|SetCurrent (.previousindex (.Value (Utilities|Map|Find (Variables|Default|GetPathfindingDataMap) (LocalVariables|GetCurrent))))))
  (bind _arrayelement (Utilities|Array|ReverseforEachLoop (LocalVariables|GetInvertedPath))
    (:LoopBody
      (Utilities|Array|Add (LocalVariables|GetRet) _arrayelement))
    (:Completed
      (return (LocalVariables|GetRet)))))

(fn ClearGenerated
  (Utilities|Map|Clear (Variables|Default|GetPathfindingDataMap))
  (Utilities|Array|Clear (Variables|Default|GetDiscoveredTileSortingCost))
  (Utilities|Array|Clear (Variables|Default|GetDiscoveredTileIndices))
  (Utilities|Array|Clear (Variables|Default|GetAnalyzedTileIndices))
  (Default|CallOnPathfindingDataCleared))

(fn DiscoverTile
  (params (TilePathData :type S%20Pathfinding%20Data%20Structure))
  (Utilities|Map|Add (Variables|Default|GetPathfindingDataMap) (.Index (Utilities|Struct|BreakS_PathfindingData TilePathData)) TilePathData)
  (CallFunction|InsertTileinDiscoveredArray)
  (Default|CallOnPathfindingDataUpdated))

(fn InsertTileinDiscoveredArray
  (params (TileData :type S%20Pathfinding%20Data%20Structure))
  (bind _discoveredtilesortingcost (Variables|Default|GetDiscoveredTileSortingCost))
  (LocalVariables|SetSortingCost (CallFunction|GetTileSortingCost TileData))
  (if (== (Utilities|Array|Length (Variables|Default|GetDiscoveredTileSortingCost)) 0)
    (Utilities|Array|Add (Variables|Default|GetDiscoveredTileSortingCost) (LocalVariables|GetSortingCost) :!label _label)
    (Utilities|Array|Add (Variables|Default|GetDiscoveredTileIndices) (.index TileData))
    (elif (>= (LocalVariables|GetSortingCost) (Utilities|Array|Get(acopy) _discoveredtilesortingcost (Utilities|Array|LastIndex _discoveredtilesortingcost)))
      (goto _label)
      (else
        (bind (_array_element _array_index) (Utilities|Array|ForEachLoopwithBreak (Variables|Default|GetDiscoveredTileSortingCost) :!label _label_2)
          (:LoopBody
            (if (>= _array_element (LocalVariables|GetSortingCost))
              (Utilities|Array|Insert (Variables|Default|GetDiscoveredTileSortingCost) (LocalVariables|GetSortingCost) _array_index)
              (Utilities|Array|Insert (Variables|Default|GetDiscoveredTileIndices) (.Index (Utilities|Struct|BreakS_PathfindingData TileData)) _array_index)
              (goto _label_2 Break))))))))

(fn GetTileSortingCost
  (params (TileData :type S%20Pathfinding%20Data%20Structure))
  (bind (_index _costtoentertile _costfromstart _minimumcosttotarget _previousindex) (Utilities|Struct|BreakS_PathfindingData TileData))
  (bind (_index_2 _costtoentertile_2 _costfromstart_2 _minimumcosttotarget_2) (Utilities|Struct|BreakS_PathfindingData TileData))
  (return (+ (* (+ _costfromstart_2 _minimumcosttotarget_2) 2) (CallFunction|IsDiagonal _index _previousindex))))

(fn IsDiagonal
  (params (Index%201 :type Int%20Point%20Structure) (Index%202 :type Int%20Point%20Structure))
  (bind _neighbors (CallFunction|GetNeighborIndexes Index%201 false))
  (return (not (Utilities|Array|ContainsItem _neighbors Index%202))))

(fn PullCheapestTilefromDiscoveredList
  (LocalVariables|SetTileIndex (Utilities|Array|Get(acopy) (Variables|Default|GetDiscoveredTileIndices)))
  (Utilities|Array|RemoveItem (Variables|Default|GetDiscoveredTileSortingCost) 0)
  (Utilities|Array|RemoveIndex (Variables|Default|GetDiscoveredTileIndices))
  (Utilities|Array|Add (Variables|Default|GetAnalyzedTileIndices) (LocalVariables|GetTileIndex))
  (return (.Value (Utilities|Map|Find (Variables|Default|GetPathfindingDataMap) (LocalVariables|GetTileIndex)))))

(fn DiscoverNextNeighbor)

(fn GetPathCost
  (params (Path :type Array%20of%20Int%20Point%20Structures))
  (LocalVariables|SetRet 0)
  (for _array_element Path
    (LocalVariables|SetRet (+ (LocalVariables|GetRet) (CallFunction|GetTileTypeMoveCost (.TileType (Utilities|Struct|BreakS_TileData (.Value (Utilities|Map|Find (Variables|/Game/Blueprints/BP_Grid.BP_Grid_C|GetGridTileMap (Variables|Default|GetGrid)) _array_element))))))))
  (return (LocalVariables|GetRet)))