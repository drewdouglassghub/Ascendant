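; BP_GridModifier is a grid marker actor with a Shape and a tile Type, such as Normal, Obstacle, a movement cost or FlyingOnly.
; Its construction script applies the shape's flat mesh and material, then tints it by Type as a filled tile.
; It also sets trace collision, with only the None type blocking Pawn, and hides the actor in game.
; The event graph has no logic.
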(event EventBeginPlay)

(event Collision|EventActorBeginOverlap
  (params (OtherActor :type Actor%20Object%20Reference)))

(event EventTick
  (params (DeltaSeconds :type Float%20%28single-precision%29)))

(fn ConstructionScript
  (bind _staticmesh (Variables|Default|GetStaticMesh))
  (bind _shape (Variables|Default|GetShape))
  (bind _staticmesh_2 (Variables|Default|GetStaticMesh))
  (bind _out_row (CallFunction|GetShapeData _shape))
  (Components|StaticMesh|SetStaticMesh _staticmesh_2 (.flatmesh _out_row))
  (Rendering|Material|SetMaterial _staticmesh_2 0 (.flatmaterial _out_row))
  (Rendering|Material|SetVectorParameterValueonMaterials _staticmesh_2 "Color" (Math|Conversions|ToVector(LinearColor) (Utilities|Select :Index (Variables|Default|GetType) :NewEnumerator0 "(R=0.958333,G=0.958333,B=0.958333,A=1.000000)" :NewEnumerator1 "(R=0.427146,G=1.000000,B=0.640438,A=0.860870)" :NewEnumerator2 "" :NewEnumerator3 "" :NewEnumerator4 "" :NewEnumerator5 "")))
  (Rendering|Material|SetScalarParameterValueonMaterials (Variables|Default|GetStaticMesh) "IsFilled" 1.0)
  (Collision|SetCollisionResponsetoChannel _staticmesh "ECC_Visibility" "ECR_Overlap")
  (Collision|SetCollisionResponsetoChannel _staticmesh "ECC_Visibility" "ECR_Block")
  (Collision|SetCollisionResponsetoChannel _staticmesh "ECC_Pawn" (select (Utilities|Enum|Equal(Enum) (Variables|Default|GetType) "NewEnumerator0") "ECR_Block" "ECR_Ignore"))
  (Rendering|SetActorHiddenInGame true))