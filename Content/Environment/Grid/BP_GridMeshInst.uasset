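; Grid mesh actor that draws cells through one InstancedStaticMesh, with instances added and removed by grid index.
; InitializeGridMeshInst sets the shared mesh and material and makes collision query-only.
; A parallel InstanceIndices array maps each grid index to its instance slot, so AddInstance replaces any existing entry and ClearInstance empties both.
; Mesh and material inputs on AddInstance are unused, and the per-instance color custom data code is disconnected.
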(event EventBeginPlay)

(event Collision|EventActorBeginOverlap
  (params (OtherActor :type Actor%20Object%20Reference)))

(event EventTick
  (params (DeltaSeconds :type Float%20%28single-precision%29)))

(fn ConstructionScript)

(fn InitializeGridMeshInst
  (params (Index :type Int%20Point%20Structure) (Transform :type Transform) (Height :type Float%20%28double-precision%29) (Mesh :type Static%20Mesh%20Object%20Reference) (Material :type Material%20Interface%20Object%20Reference))
  (bind _instancedstaticmesh (Variables|Default|GetInstancedStaticMesh))
  (Components|StaticMesh|SetStaticMesh _instancedstaticmesh Mesh)
  (Rendering|Material|SetMaterial _instancedstaticmesh 0 Material)
  (Collision|SetCollisionEnabled _instancedstaticmesh "QueryOnly"))

(fn ClearInstance
  (Components|InstancedStaticMesh|ClearInstances (Variables|Default|GetInstancedStaticMesh))
  (Utilities|Array|Clear (Variables|Default|GetInstanceIndices)))

(fn RemoveInstance
  (params (Index :type Int%20Point%20Structure%20%28by%20ref%29))
  (bind _instanceindices (Variables|Default|GetInstanceIndices))
  (if (Utilities|Array|ContainsItem _instanceindices Index)
    (Class|InstancedStaticMeshComponent|RemoveInstance (Variables|Default|GetInstancedStaticMesh) (Utilities|Array|FindItem _instanceindices Index))
    (Utilities|Array|RemoveItem (Variables|Default|GetInstanceIndices) Index)))

(fn AddInstance
  (params (Index :type Int%20Point%20Structure) (Transform :type Transform) (Mesh :type Static%20Mesh%20Object%20Reference) (Material :type Material%20Instance%20Object%20Reference))
  (CallFunction|RemoveInstance Index)
  (Components|InstancedStaticMesh|AddInstance (Variables|Default|GetInstancedStaticMesh) Transform true)
  (Utilities|Array|Add (Variables|Default|GetInstanceIndices) Index))