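; BP_PlacementGrid is an unfinished placement grid with helpers for tile data, visual updates, cursor picking and ground snapping.
; Cursor picking falls back from channel traces to a mouse-ray intersection with the grid's plane.
; Tile corners are computed only for a six-sided shape, then line-traced for ground location and normal.
; Nearly all logic is disconnected from its entry points; only TraceForGround's sphere trace runs, with its results unused.
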(event EventBeginPlay)

(event Collision|EventActorBeginOverlap
  (params (OtherActor :type Actor%20Object%20Reference)))

(event EventTick
  (params (DeltaSeconds :type Float%20%28single-precision%29)))

(fn ConstructionScript)

(fn AddGridTile
  (params (Data :type S%20Tile%20Data%20Structure)))

(fn DestroyGrid)

(fn GetCursorLocation
  (params (PlayerIndex :type Integer)))

(fn GetTileRotation
  (params (GridIndex :type Int%20Point%20Structure) (GridIndex_X :type Integer) (GridIndex_Y :type Integer)))

(fn TraceforGround
  (params (Location :type Vector) (Index :type Int%20Point%20Structure))
  (bind _outhits (Collision|MultiSphereTraceByChannel "0, 0, 0" "0, 0, 0" (LocalVariables|GetRadius) "TraceTypeQuery3" false 0 "None")))

(fn CalculateCenterBottomLeft
  ;[1 1 1] Square
)

(fn GetTileLocation
  (params (GridIndex :type Int%20Point%20Structure)))

(fn GetTileCorners
  (params (HexCenter :type Vector) (HexRadius :type Float%20%28double-precision%29) (Index :type Int%20Point%20Structure))
  ;[0.15 0.15 0.15 0.5] Comment
)

(fn GetTileCornerArrays
  (params (GridIndex :type Int%20Point%20Structure) (GridIndex_X :type Integer) (GridIndex_Y :type Integer)))