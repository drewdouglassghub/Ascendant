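; BP_Grid is a square tile grid actor, apparently for building placement, with tile data including a BuildingID.
; SpawnGrid clears and rebuilds tiles around a center, sized by the footprint SetFootprintFromBounds computes rather than its TileCount input.
; Tiles are stored in GridTileMap and drawn by a child BP_GridVisual.
; Tile height comes from the under-cursor hit; TraceForGround is uncalled here, and hexagon logic is disconnected.
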(event EventBeginPlay)

(event Collision|EventActorBeginOverlap
  (params (OtherActor :type Actor%20Object%20Reference)))

(event EventTick
  (params (DeltaSeconds :type Float%20%28single-precision%29)))

(fn ConstructionScript
  (bind _asbp_game_mode (Utilities|Casting|CastToBP_GameMode (Game|GetGameMode)))
  (Variables|Default|SetGame%20Mode _asbp_game_mode)
  (bind _outactors (Actor|GetAllActorsOfClass "/Game/Core/Blueprints/Managers/BP_PlacementManager.BP_PlacementManager_C"))
  (Variables|Default|SetPlacement%20Manager (Utilities|Array|Get(acopy) _outactors))
  (bind _asbp_grid_visual (Utilities|Casting|CastToBP_GridVisual (Variables|/Script/Engine.ChildActorComponent|GetChildActor (Variables|Default|GetChildActor_GridVisual)))
    (:then
      (Variables|Default|SetGridVisual _asbp_grid_visual))
    (:CastFailed
      (Development|PrintString "visual cast fail"))))

(fn GetTileRotation
  (params (GridIndex :type Int%20Point%20Structure))
  (return "0, 0, 0"))

(fn GetTileCorners
  (params (HexCenter :type Vector) (HexRadius :type Float%20%28double-precision%29) (Index :type Int%20Point%20Structure))
  ;[0.15 0.15 0.15 0.5] Comment
)

(fn IsIndexValid
  (params (Index :type Int%20Point%20Structure))
  (if (Utilities|Map|Contains (Variables|Default|GetGridTileMap) Index)
    (return true)))

(fn GetTileScale
  (bind _tile_size (Variables|Default|GetTile%20Size))
  (return (Math|Vector|MakeVector (.x _tile_size) (.y _tile_size) 0.0)))

(fn AddGridTile
  (params (Data :type S%20Tile%20Data%20Structure))
  (bind _output_get (LocalVariables|Setindex (.index Data)))
  (Utilities|Map|Add (Variables|Default|GetGridTileMap) _output_get (Utilities|Struct|MakeS_TileData _output_get (.transform Data) (.tilemesh Data) (.tilematerial Data) (.worldlocation Data) (.tileinst Data) (.buildingid Data)))
  (Default|UpdateTileVisual (Variables|Default|GetGridVisual) Data)
  (Default|CallOnTileDataUpdated))

(fn TraceforGround
  (params (Location :type Vector) (Index :type Int%20Point%20Structure))
  (bind _childactor_gridvisual (Variables|Default|GetChildActor_GridVisual))
  (bind (_origin _boxextent _sphereradius) (Collision|GetComponentBounds _childactor_gridvisual))
  (Variables|Default|SetShapeRadius (/ (.x (Variables|Default|GetTile%20Size)) 5.0))
  (bind (_outhits _returnvalue) (Collision|MultiSphereTraceByChannel (+ Location "") (- Location "0.000000,0.000000,60000.000000") (LocalVariables|GetRadius) "TraceTypeQuery3" false 0 "None" true "(R=0.000000,G=1.000000,B=0.000000,A=1.000000)" "(R=0.994792,G=0.022352,B=0.012378,A=1.000000)"))
  (if _returnvalue
    (for _array_element _outhits
      (if (Variables|Default|GetIsHeightFound)
        (LocalVariables|SetRetZ (Math|Float|SnapToGrid(Float) (+ _sphereradius (.z (.ImpactPoint (Collision|BreakHitResult _array_element)))) (.x _boxextent)))
        (else
          (Development|PrintString "Height not found"))))
    (return (Math|Vector|MakeVector (.x Location) (.y Location) (LocalVariables|GetRetZ)))
    (else
      (return Location))))

(fn CalculateCenterBottomLeft
  (bind _center_location (Variables|Default|GetCenter%20Location))
  (bind _tile_count (Variables|Default|GetTile%20Count))
  (bind _tile_size (Variables|Default|GetTile%20Size))
  ;[1 1 1] Square
  (Variables|Default|SetHalfX (/ (* (.x _tile_size) (.x _tile_count)) 2.0))
  (Variables|Default|SetHalfY (/ (* (.y _tile_size) (.y _tile_count)) 2.0))
  (return _center_location (- _center_location (Math|Vector|MakeVector (- (Variables|Default|GetHalfX) (/ (.x (Variables|Default|GetTile%20Size)) 2.0)) (- (Variables|Default|GetHalfY) (/ (.x (Variables|Default|GetTile%20Size)) 2.0)) 1.0))))

(fn DestroyGrid
  (Utilities|Map|Clear (Variables|Default|GetGridTileMap))
  (Default|DestroyGridVisual (Variables|Default|GetGridVisual))
  (Default|CallOnGridDestroyed))

(fn GetTileLocation
  (params (GridIndex :type Int%20Point%20Structure))
  (bind _tile_size (Variables|Default|GetTile%20Size))
  (bind _gridbottomleftlocation (Variables|Default|GetGridBottomLeftLocation))
  (return (Math|Vector|MakeVector (+ (.x _gridbottomleftlocation) (* (.x GridIndex) (.x _tile_size))) (+ (.y _gridbottomleftlocation) (* (.y GridIndex) (.y _tile_size))) 0.0)))

(fn SpawnGrid
  (params (CenterLocation :type Vector) (TileSize :type Vector) (TileCount :type Int%20Point%20Structure))
  ;[1 1 1] Set Variables for Grid
  (Development|PrintString "SpawnGrid")
  (Variables|Default|SetCenter%20Location CenterLocation)
  (Variables|Default|SetTile%20Size TileSize)
  (Variables|Default|SetTile%20Count (Utilities|Struct|MakeIntPoint (Variables|Default|GetFootprintX) (Variables|Default|GetFootprintY)))
  (Utilities|FlowControl|Sequence
    (:then_0
      (CallFunction|DestroyGrid)
      ;[1 1 1] Respawn Current Grid
      (Default|InitializeGridVisual (Variables|Default|GetGridVisual) self)
      (bind (_center _bottom_left) (CallFunction|CalculateCenterBottomLeft))
      (Variables|Default|SetCenter%20Location _center)
      (Variables|Default|SetGridBottomLeftLocation _bottom_left)
      ;[1 1 1] X - Grid For Loop
      (for _index (range 0 (- (.x (Variables|Default|GetTile%20Count)) 1))
        (LocalVariables|SetX _index)
        ;[1 1 1] Y - Grid For Loop
        (for _index_2 (range 0 (- (Math|Float|Round (Math|Conversions|ToFloat(Integer) (.y (Variables|Default|GetTile%20Count)))) 1))
          (LocalVariables|SetY _index_2)
          ;[1 1 1] Trace for ground accommodates grid environment of different heights.  Also sets transform of tile.
          (LocalVariables|SetIndex (Utilities|Struct|MakeIntPoint (LocalVariables|GetX) (LocalVariables|GetY)))
          (CallFunction|AddGridTile (Utilities|Struct|MakeS_TileData (LocalVariables|GetIndex) (Math|Transform|MakeTransform (.Location (Math|Transform|BreakTransform (Math|Transform|MakeTransform (Math|Vector|MakeVector (.x (CallFunction|GetTileLocation (LocalVariables|GetIndex))) (.y (CallFunction|GetTileLocation (LocalVariables|GetIndex))) (.z (.ImpactPoint (Collision|BreakHitResult (.HitResult (Game|Player|GetHitResultUnderCursorbyChannel (.AsBP%20Player%20Controller (Utilities|Casting|CastToBP_PlayerController (Game|GetPlayerController 0))) "TraceTypeQuery4" true))))))))) (.Rotation (Math|Transform|BreakTransform (Math|Transform|MakeTransform (Math|Vector|MakeVector (.x (CallFunction|GetTileLocation (LocalVariables|GetIndex))) (.y (CallFunction|GetTileLocation (LocalVariables|GetIndex))) (.z (.ImpactPoint (Collision|BreakHitResult (.HitResult (Game|Player|GetHitResultUnderCursorbyChannel (.AsBP%20Player%20Controller (Utilities|Casting|CastToBP_PlayerController (Game|GetPlayerController 0))) "TraceTypeQuery4" true))))))))) (.Scale (Math|Transform|BreakTransform (Math|Transform|MakeTransform (Math|Vector|MakeVector (.x (CallFunction|GetTileLocation (LocalVariables|GetIndex))) (.y (CallFunction|GetTileLocation (LocalVariables|GetIndex))) (.z (.ImpactPoint (Collision|BreakHitResult (.HitResult (Game|Player|GetHitResultUnderCursorbyChannel (.AsBP%20Player%20Controller (Utilities|Casting|CastToBP_PlayerController (Game|GetPlayerController 0))) "TraceTypeQuery4" true)))))))))) "/Game/Environment/Meshes/Grid/Square/SM_Grid_SquareFlat.SM_Grid_SquareFlat" "/Game/Environment/Meshes/Grid/Square/MI_FlatSquareValid.MI_FlatSquareValid" (.Location (Math|Transform|BreakTransform (Math|Transform|MakeTransform (Math|Vector|MakeVector (.x (CallFunction|GetTileLocation (LocalVariables|GetIndex))) (.y (CallFunction|GetTileLocation (LocalVariables|GetIndex))) (.z (.ImpactPoint (Collision|BreakHitResult (.HitResult (Game|Player|GetHitResultUnderCursorbyChannel (.AsBP%20Player%20Controller (Utilities|Casting|CastToBP_PlayerController (Game|GetPlayerController 0))) "TraceTypeQuery4" true))))))))) 0 0)))))
    (:then_1
      (Development|PrintString "Grid Built")
      (Default|CallOnGridBuild))))

(fn SetFootprintfromBounds
  (params (Origin :type Vector) (BoxExtent :type Vector) (TileSize :type Float%20%28double-precision%29))
  (Variables|Default|SetMin (- Origin BoxExtent))
  (Variables|Default|SetMax (+ Origin BoxExtent))
  (bind _output_get (Variables|Default|SetFootprintX (+ (- (Math|Float|Floor (/ (.x (Variables|Default|GetMax)) (.x (Variables|Default|GetTile%20Size)))) (Math|Float|Floor (/ (.x (Variables|Default|GetMin)) (.x (Variables|Default|GetTile%20Size))))) 1)))
  (CallFunction|LogInteger "X " _output_get)
  (bind _output_get_2 (Variables|Default|SetFootprintY (+ (- (Math|Float|Floor (/ (.y (Variables|Default|GetMax)) (.x (Variables|Default|GetTile%20Size)))) (Math|Float|Floor (/ (.y (Variables|Default|GetMin)) (.y (Variables|Default|GetTile%20Size))))) 1)))
  (CallFunction|LogInteger "Y " _output_get_2))