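; Building grid mesh actor that shows an instanced static mesh as an invalid-square highlight while something overlaps it.
; Begin overlap prints a debug message, makes the component visible and applies MI_FlatSquareInvalid; end overlap hides it and sets that same material again.
; Visibility and material apply to the whole instanced component rather than individual instances.
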(event OnComponentBeginOverlap(InstancedStaticMesh)
  (params (OverlappedComponent :type Primitive%20Component%20Object%20Reference) (OtherActor :type Actor%20Object%20Reference) (OtherComp :type Primitive%20Component%20Object%20Reference) (OtherBodyIndex :type Integer) (bFromSweep :type Boolean) (SweepResult :type Hit%20Result%20Structure%20%28by%20ref%29))
  (Development|PrintString "Overlapping")
  (Rendering|SetVisibility OverlappedComponent true false)
  (Rendering|Material|SetMaterial (Variables|Default|GetInstancedStaticMesh) 0 "/Game/Environment/Meshes/Grid/Square/MI_FlatSquareInvalid.MI_FlatSquareInvalid"))

(event OnComponentEndOverlap(InstancedStaticMesh)
  (params (OverlappedComponent :type Primitive%20Component%20Object%20Reference) (OtherActor :type Actor%20Object%20Reference) (OtherComp :type Primitive%20Component%20Object%20Reference) (OtherBodyIndex :type Integer))
  (Rendering|SetVisibility OverlappedComponent false false)
  (Rendering|Material|SetMaterial (Variables|Default|GetInstancedStaticMesh) 0 "/Game/Environment/Meshes/Grid/Square/MI_FlatSquareInvalid.MI_FlatSquareInvalid"))

(event EventBeginPlay
  (|CallParentFunction) ; This node is disabled and will not be called.\nDrag off pins to build functionality.
)

(event Collision|EventActorBeginOverlap
  (params (OtherActor :type Actor%20Object%20Reference))
  (|CallParentFunction OtherActor) ; This node is disabled and will not be called.\nDrag off pins to build functionality.
)

(event EventTick
  (params (DeltaSeconds :type Float%20%28single-precision%29))
  (|CallParentFunction DeltaSeconds) ; This node is disabled and will not be called.\nDrag off pins to build functionality.
)

(fn ConstructionScript
  (|CallParentFunction))