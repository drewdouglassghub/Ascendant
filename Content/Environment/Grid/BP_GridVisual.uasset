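; BP_GridVisual is the visual layer for a tile grid, drawing tiles through a BP_GridMeshInst child actor.
; It caches that child on construction and initializes it from tile transform, height, mesh and material data.
; Tile updates remove and re-add the instance by index, and teardown clears all instances.
; A separate function raises the child actor above the root by a ground offset.
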(event EventBeginPlay)

(event Collision|EventActorBeginOverlap
  (params (OtherActor :type Actor%20Object%20Reference)))

(event EventTick
  (params (DeltaSeconds :type Float%20%28single-precision%29)))

(fn ConstructionScript
  (bind _asbp_grid_mesh_inst (Utilities|Casting|CastToBP_GridMeshInst (Variables|/Script/Engine.ChildActorComponent|GetChildActor (Variables|Default|GetChildActor_GridMeshInst))))
  (Variables|Default|SetGridMeshInst _asbp_grid_mesh_inst))

(fn InitializeGridVisual
  (params (Grid :type BP%20Grid%20Object%20Reference))
  (Variables|Default|SetGrid Grid)
  (Variables|Default|SetGridMeshInst (.AsBP%20Grid%20Mesh%20Inst (Utilities|Casting|CastToBP_GridMeshInst (Variables|/Script/Engine.ChildActorComponent|GetChildActor (Variables|Default|GetChildActor_GridMeshInst)))))
  (bind _tileinst (Default|InitializeGridMeshInst (Variables|Default|GetGridMeshInst) (.index (Variables|Default|GetTileData)) (.transform (Variables|Default|GetTileData)) (.z (.worldlocation (Variables|Default|GetTileData))) (.tilemesh (Variables|Default|GetTileData)) (.tilematerial (Variables|Default|GetTileData)) false))
  (Variables|Default|SetTileData (Utilities|Struct|MakeS_TileData (.index (Variables|Default|GetTileData)) (.transform (Variables|Default|GetTileData)) (.tilemesh (Variables|Default|GetTileData)) (.tilematerial (Variables|Default|GetTileData)) (Math|Vector|MakeVector 0.0 0.0 (.z (.worldlocation (Variables|Default|GetTileData)))) _tileinst 0)))

(fn SetOffsetfromGround
  (params (Offset :type Float%20%28double-precision%29))
  (bind _defaultsceneroot (Variables|Default|GetDefaultSceneRoot))
  (bind _returnvalue (Transformation|GetWorldLocation _defaultsceneroot))
  (Variables|Default|SetOffsetFromGround Offset)
  (Transformation|SetWorldLocation (Variables|Default|GetChildActor_GridMeshInst) (Math|Vector|MakeVector (.x _returnvalue) (.y _returnvalue) (+ (.z _returnvalue) (Variables|Default|GetOffsetFromGround))) false false))

(fn UpdateTileVisual
  (params (Data :type S%20Tile%20Data%20Structure))
  (bind _gridmeshinst (Variables|Default|GetGridMeshInst))
  (Variables|Default|SetTileData Data)
  (Default|RemoveInstance _gridmeshinst (.index (Variables|Default|GetTileData)))
  (Default|AddInstance _gridmeshinst (.index (Variables|Default|GetTileData)) (.transform (Variables|Default|GetTileData)) (.tilemesh (Variables|Default|GetTileData)) (.tilematerial (Variables|Default|GetTileData)) (.worldlocation (Variables|Default|GetTileData)) (.buildingid (Variables|Default|GetTileData))))

(fn SetGridLowestZ
  (params (GridLowestZ :type Float%20%28double-precision%29))
  (Variables|Default|SetGrid%20Lowest%20Z GridLowestZ))

(fn DestroyGridVisual
  (bind _gridmeshinst (Variables|Default|GetGridMeshInst))
  (Utilities|IsValid _gridmeshinst
    (:Is%20Valid
      (Default|ClearInstance _gridmeshinst))
    (:Is%20Not%20Valid
      (CallFunction|LogText "instance mesh not valid"))))